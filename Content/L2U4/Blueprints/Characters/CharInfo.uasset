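; CharInfo is a character data container that exposes a character's stored profile and state through getter functions.
; It covers identity (ID, name, class, preset name), progression (level, experience), transform (location, rotation) and vitals (health, mana).
; Each getter returns its member variable directly, and the graphs contain no setters, events or other logic.
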(fn `GetCharClass`
  (returns (ReturnValue :type "/Game/L2U4/Data/Enum/E_CharClass Enum"))
  (return (`self.CharClass`)))

(fn `GetCharExperience`
  (returns (ReturnValue :type Integer))
  (return (`self.Experience`)))

(fn `GetCharHealth`
  (returns (ReturnValue :type Integer))
  (return (`self.Health`)))

(fn `GetCharID`
  (returns (ReturnValue :type Integer))
  (return (`self.ID`)))

(fn `GetCharLevel`
  (returns (ReturnValue :type Integer))
  (return (`self.Level`)))

(fn `GetCharLocation`
  (returns (Location :type "Vector Structure"))
  (return (`self.Location`)))

(fn `GetCharMana`
  (returns (ReturnValue :type Integer))
  (return (`self.Mana`)))

(fn `GetCharName`
  (returns (ReturnValue :type String))
  (return (`self.Name`)))

(fn `GetCharRotation`
  (returns (Rotation :type "Rotator Structure"))
  (return (`self.Rotation`)))

(fn `GetPresetName`
  (returns (ReturnValue :type Name))
  (return (`self.PresetName`)))