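; PlayerChar is the player character Blueprint, providing basic movement and camera-look controls.
; MoveForward and MoveRight axes add movement along forward and right vectors built from control-rotation yaw only, so pitch does not affect direction.
; MouseX and MouseY drive controller yaw and negated pitch only while the right mouse button is held, tracked by an RMBPressed flag.
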(event `InputAxis|MoveForward`
  (params (AxisValue :type "Float (single-precision)"))
  (bind (_returnvalue_roll _returnvalue_pitch _returnvalue_yaw) (`KismetMathLibrary.BreakRotator` (`self.GetControlRotation`)))
  (`self.AddMovementInput` (`KismetMathLibrary.GetForwardVector` (`KismetMathLibrary.MakeRotator` 0.0 0.0 _returnvalue_yaw)) AxisValue))

(event `InputAxis|MoveRight`
  (params (AxisValue :type "Float (single-precision)"))
  (bind (_returnvalue_roll _returnvalue_pitch _returnvalue_yaw) (`KismetMathLibrary.BreakRotator` (`self.GetControlRotation`)))
  (`self.AddMovementInput` (`KismetMathLibrary.GetRightVector` (`KismetMathLibrary.MakeRotator` 0.0 0.0 _returnvalue_yaw)) AxisValue))

(event `InputAxisKey|MouseX`
  (params (AxisValue :type "Float (single-precision)"))
  (if (`self.RMB Pressed?`)
    (`self.AddControllerYawInput` AxisValue)))

(event `InputAxisKey|MouseY`
  (params (AxisValue :type "Float (single-precision)"))
  (if (`self.RMB Pressed?`)
    (`self.AddControllerPitchInput` (* AxisValue -1.0))))

(event `Key|RightMouseButton`
  (params (Key :type "Key Structure"))
  (:`Pressed`
    (set `self.RMB Pressed?` true))
  (:`Released`
    (set `self.RMB Pressed?` false)))

(fn `UserConstructionScript`
  (`parent.UserConstructionScript`))