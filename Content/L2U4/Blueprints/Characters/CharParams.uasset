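; CharParams is a character Blueprint that sets up the character's stats and appearance from player-state data.
; Shortly after BeginPlay, a fixed delay elapses, then it reads the character info message from PlayerState and initializes the ACCharacterParams component with health, mana, level, experience and name.
; The message's preset name selects a DT_CharPreset row, which supplies the skeletal mesh and animation class.
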(event `self.ReceiveBeginPlay`
  (bind _mesh (`self.Mesh`))
  (bind _charinfo (`self.CharInfo`))
  (`KismetSystemLibrary.Delay` 0.5)
  (bind _returninfo (message `/Game/L2U4/Blueprints/PlayerState/BPI_PS_Params.GetCurrentCharInfo` (`self.PlayerState`)))
  (set `self.CharInfo` _returninfo)
  (`/Game/L2U4/Blueprints/Components/AC_CharacterParams.InitializeCharParams` (`self.AC_CharacterParams`) (`/Game/L2U4/Blueprints/Characters/CharInfo.GetCharHealth` _charinfo) (`/Game/L2U4/Blueprints/Characters/CharInfo.GetCharMana` _charinfo) (`/Game/L2U4/Blueprints/Characters/CharInfo.GetCharLevel` _charinfo) (`/Game/L2U4/Blueprints/Characters/CharInfo.GetCharExperience` _charinfo) (`/Game/L2U4/Blueprints/Characters/CharInfo.GetCharName` _charinfo))
  (bind _returnvalue (`|GetDataTableRow` "/Game/L2U4/Data/Datatables/DT_CharPreset.DT_CharPreset" (`/Game/L2U4/Blueprints/Characters/CharInfo.GetPresetName` (`self.CharInfo`)))
    (:`then`
      (bind (_mesh_2 _healthpoint _manapoint _currentcp _presetlevelname _animinstance) (break `/Game/L2U4/Data/Struct/S_CharPresset` _returnvalue))
      (`SkinnedMeshComponent.SetSkinnedAssetAndUpdate` _mesh _mesh_2 true)
      (`SkeletalMeshComponent.SetAnimInstanceClass` _mesh _animinstance))))

(fn `UserConstructionScript`
  (`parent.UserConstructionScript`))