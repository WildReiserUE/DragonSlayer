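; Player controller layer that handles switching the player's current character and provides helpers to spawn arena and local characters.
; A change request takes a busy lock, validates the index, then applies through PlayerState on authority or forwards to the server from a client.
; The response clears the lock, relays from server to client, and reports errors or refreshes the main menu character list.
; Arena characters spawn only with authority, while local characters spawn by index or row name.
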(event `Change Current Char on server`
  (params (Index :type Integer))
  (`self.ChangeCurrent_Char` Index))

(event `self.ChangeCurrent_Char`
  (params (Index :type Integer))
  (bind _returninfo (`self.GetCharByIndex` Index))
  (if (not (`self.HasBusy`))
    (`self.ChangeBusy` true)
    (`/Engine/EditorBlueprintResources/StandardMacros.IsValid` _returninfo
      (:`Is Valid`
        (if (== (`self.GetCurrentCharInfo`) _returninfo)
          (`self.Response Change Current Char` "Char already used")
          (else
            (`/Engine/EditorBlueprintResources/ActorMacros.Switch Has Authority`
              (:`Authority`
                (message `/Game/L2U4/Blueprints/PlayerState/BPI_PS_Params.ChangeCurrentChar` (`self.PlayerState`) Index)
                (`self.Response Change Current Char` ""))
              (:`Remote`
                (`self.Change Current Char on server` Index))))))
      (:`Is Not Valid`
        (`self.Response Change Current Char` "Char Not Found")))))

(event `Response Change Current Char`
  (params (ErrorMessage :type String))
  (`self.ChangeBusy` false)
  (if (> (`KismetStringLibrary.Len` ErrorMessage) 0)
    (`self.RequestErrorMessage` ErrorMessage)
    (`/Engine/EditorBlueprintResources/ActorMacros.Switch Has Authority`
      (:`Authority`
        (`self.Response Change Current Char on client` ErrorMessage)))
    (else
      (`/Engine/EditorBlueprintResources/ActorMacros.Switch Has Authority`
        (:`Authority`
          (`self.Response Change Current Char on client` ErrorMessage))
        (:`Remote`
          (bind _returnwidget (message `/Game/L2U4/Blueprints/Controller/BPI_PC_MainMenu.GetMainMenuUI` self))
          (message `/Game/L2U4/UI/UII/WBPI_MainMenu.UpdateCharList` _returnwidget))))))

(event `Response Change Current Char on client`
  (params (ErrorMessage :type String))
  (`self.Response Change Current Char` ErrorMessage))

(fn `SpawnArenaChar`
  (params (SpawnLocation :type "Vector Structure") (SpawnRotation :type "Rotator Structure") (CharInfo :type "/Game/L2U4/Blueprints/Characters/CharInfo Object Reference"))
  (returns (ReturnChar :type "Character Object Reference"))
  (`/Engine/EditorBlueprintResources/ActorMacros.Switch Has Authority`
    (:`Authority`
      (bind _returnvalue (`|SpawnActorFromClass` "/Game/L2U4/Blueprints/Characters/PlayerChar.PlayerChar_C" (`KismetMathLibrary.MakeTransform` SpawnLocation SpawnRotation) "AlwaysSpawn" "OverrideRootScale" null CharInfo "0" null))
      (return _returnvalue))))

(fn `SpawnLocalChar`
  (params (SpawnTransform :type "Transform Structure") (CharIndex :type Integer))
  (returns (ReturnChar :type "Character Object Reference"))
  (bind _returnvalue (`|SpawnActorFromClass` "/Game/L2U4/Blueprints/Characters/LocalChar.LocalChar_C" SpawnTransform "AlwaysSpawn" "OverrideRootScale" null (`KismetStringLibrary.Conv_StringToName` (`KismetStringLibrary.Conv_IntToString` CharIndex)) null))
  (return _returnvalue))

(fn `SpawnLocalCharByRowName`
  (params (SpawnTransform :type "Transform Structure") (RowName :type Name))
  (returns (ReturnChar :type "Character Object Reference"))
  (bind _returnvalue (`|SpawnActorFromClass` "/Game/L2U4/Blueprints/Characters/LocalChar.LocalChar_C" SpawnTransform "AlwaysSpawn" "OverrideRootScale" null RowName null))
  (return _returnvalue))

(fn `UserConstructionScript`
  (`parent.UserConstructionScript`))