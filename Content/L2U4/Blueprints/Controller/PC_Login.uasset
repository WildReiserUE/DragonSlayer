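; PC_Login is a login player controller that checks a username and password against the user list held by the game mode.
; UserLogin forwards credentials to UserLoginOnServer, which loops through the users, breaking at the first matching username.
; An empty list or missing user triggers LoginErrorToClient, which shows a W_Dialig error widget.
; The password comparison has no actions wired, so neither wrong passwords nor successful logins produce a response.
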(event `/Game/L2U4/Blueprints/Controller/BPI_PC_Login.UserLogin`
  (params (User :type String) (Pass :type String))
  (`self.User login on server` User Pass))

(event `User login on server`
  (params (User :type String) (Pass :type String))
  (bind _returnvalue (message `/Game/L2U4/Blueprints/GameMods/BPI_GM_Login.GetUsers` (`GameplayStatics.GetGameMode`)))
  (bind _returnarray (message `/Game/L2U4/SaveGames/BPI_SG_Users.GetUsers` _returnvalue))
  (if (> (`KismetArrayLibrary.Array_Length` _returnarray) 0)
    (for (_array_element _array_index) _returnarray
      (bind (_username _password) (break `/Game/L2U4/SaveGames/S_Users` _array_element))
      (if (`KismetStringLibrary.NotEqual_StrStr` _username User)
        (if (== _array_index (`KismetArrayLibrary.Array_LastIndex` _returnarray))
          (`self.LoginError to client` "User Not Found"))
        (else
          (`|ExecutionSequence`
            (:`then_0`
              (break))
            (:`then_1`
              (if (`KismetStringLibrary.NotEqual_StrStr` _password Pass)
                _))))))
    (else
      (`self.LoginError to client` "User Not Found"))))

(event `LoginError to client`
  (params (Message :type Text))
  (bind _returnvalue (`|CreateWidget` "/Game/L2U4/UI/W_Dialig.W_Dialig_C" self "Login Error" Message))
  (`UserWidget.AddToViewport` _returnvalue 0))

(fn `UserConstructionScript`
  (`parent.UserConstructionScript`))