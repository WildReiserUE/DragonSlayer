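; Base PlayerController that watches loading progress and exposes character info and a busy flag.
; Once OpenLoadingProgress opens a gate, non-authority Tick polls PlayerState until progress reaches 100, then calls client and server completion events and closes the gate.
; Character lookups forward to PlayerState through message calls.
; The completion events and RequestErrorMessage are empty here.
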(event `self.ReceiveTick`
  (params (DeltaSeconds :type "Float (single-precision)"))
  (bind _playerstate (`self.PlayerState`))
  (`/Engine/EditorBlueprintResources/ActorMacros.Switch Has Authority`
    (:`Remote`
      (`/Engine/EditorBlueprintResources/StandardMacros.Gate` true :!label _label
        (:`Exit`
          (`/Engine/EditorBlueprintResources/StandardMacros.IsValid` _playerstate
            (:`Is Valid`
              (bind _returnvalue (message `/Game/L2U4/Blueprints/PlayerState/BPI_PS_Base.GetLoadingProgress` _playerstate))
              (if (>= _returnvalue 100)
                (`self.Loading Progress Complete on Client`)
                (`self.Loading Progress Complete on Server`)
                (goto _label :!via `Close`)))))))))

(event `Open Loading Progress`
  (goto _label :!via `Open`))

(event `Loading Progress Complete on Server`)

(event `Loading Progress Complete on Client`)

(fn `ChangeBusy`
  (params (bisBusy :type Boolean))
  (set `self.bisBusy` bisBusy))

(fn `GetCharByIndex`
  (params (Index :type Integer))
  (returns (ReturnInfo :type "/Game/L2U4/Blueprints/Characters/CharInfo Object Reference"))
  (bind _returninfo (message `/Game/L2U4/Blueprints/PlayerState/BPI_PS_Params.GetCharByIndex` (`self.PlayerState`) Index))
  (return _returninfo))

(fn `GetCurrentCharInfo`
  (returns (ReturnInfo :type "/Game/L2U4/Blueprints/Characters/CharInfo Object Reference"))
  (bind _returninfo (message `/Game/L2U4/Blueprints/PlayerState/BPI_PS_Params.GetCurrentCharInfo` (`self.PlayerState`)))
  (return _returninfo))

(fn `HasBusy`
  (returns (bisBusy :type Boolean))
  (return (`self.bisBusy`)))

(fn `RequestErrorMessage`
  (params (Message :type "String (by ref)")))

(fn `UserConstructionScript`)