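; Player controller for the world that brings the player's current character into play after loading.
; On BeginPlay it opens a loading progress display where cosmetic events can run.
; When loading completes on the server, it spawns an arena character from valid current character info at that info's location and rotation, possesses it and shows the mouse cursor.
; The client-side completion event is empty, and stored health is not applied here.
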(event `self.ReceiveBeginPlay`
  (`parent.ReceiveBeginPlay`)
  (`/Engine/EditorBlueprintResources/StandardMacros.Can Execute Cosmetic Events`
    (:`True`
      (`self.Open Loading Progress`))))

(event `self.Loading Progress Complete on Client`)

(event `self.Loading Progress Complete on Server`
  (bind _returninfo (`self.GetCurrentCharInfo`))
  (`/Engine/EditorBlueprintResources/StandardMacros.IsValid` _returninfo
    (:`Is Valid`
      (bind _returnchar (`self.SpawnArenaChar` (`/Game/L2U4/Blueprints/Characters/CharInfo.GetCharLocation` _returninfo) (`/Game/L2U4/Blueprints/Characters/CharInfo.GetCharRotation` _returninfo) _returninfo))
      (`self.Possess` _returnchar)
      (set `self.bShowMouseCursor` true))))

(fn `UserConstructionScript`
  (`parent.UserConstructionScript`))