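; Main menu player controller that runs the loading progress, creates the menu widgets and handles character creation requests.
; Once client loading completes, it builds and caches the main menu, a collapsed select/create character screen and the create character widget.
; New character data is busy-guarded and forwarded to the server, which adds it through PlayerState.
; The result returns to the client, clearing busy and printing any error.
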(event `self.ReceiveBeginPlay`
  (`/Engine/EditorBlueprintResources/StandardMacros.Can Execute Cosmetic Events`
    (:`True`
      (`self.Open Loading Progress`))))

(event `self.Loading Progress Complete on Client`
  (bind _returnvalue (`|CreateWidget` "/Game/L2U4/UI/2Lobby/W_MainMenu.W_MainMenu_C" self))
  (`UserWidget.AddToViewport` _returnvalue 0)
  (set `self.MainMenuWidget` _returnvalue)
  (bind _returnvalue_2 (`|CreateWidget` "/Game/L2U4/UI/2Lobby/W_SelectCreateChar.W_SelectCreateChar_C" self))
  (`Widget.SetVisibility` _returnvalue_2 "Collapsed")
  (`UserWidget.AddToViewport` _returnvalue_2 0)
  (set `self.SelectCreateCharWidget` _returnvalue_2)
  (bind _returnvalue_3 (`|CreateWidget` "/Game/L2U4/UI/2Lobby/W_CreateChar.W_CreateChar_C" self))
  (set `self.CreateCharWidget` _returnvalue_3))

(event `self.AddCharData`
  (params (CharInfoData :type "/Game/L2U4/Data/Struct/S_CharInfo Structure (by ref)"))
  (if (not (`self.HasBusy`))
    (`self.ChangeBusy` true)
    (`/Engine/EditorBlueprintResources/ActorMacros.Switch Has Authority`
      (:`Authority`
        (bind _result (message `/Game/L2U4/Blueprints/PlayerState/BPI_PS_Params.AddChar` (`self.PlayerState`) CharInfoData true))
        (if _result
          (`self.Response Add Char` "")
          (else
            (`self.Response Add Char` "ERROR to CLIENT"))))
      (:`Remote`
        (`self.Add char data to server` CharInfoData)))))

(event `Add char data to server`
  (params (CharInfoData :type "/Game/L2U4/Data/Struct/S_CharInfo Structure"))
  (`self.AddCharData` CharInfoData))

(event `Response Add Char`
  (params (ErrorMessage :type String))
  (`self.ChangeBusy` false)
  (if (== (`KismetStringLibrary.Len` ErrorMessage) 0)
    (`/Engine/EditorBlueprintResources/ActorMacros.Switch Has Authority`
      (:`Authority`
        (`self.Response Add Char on client` ErrorMessage)))
    (else
      (`KismetSystemLibrary.PrintString` ErrorMessage true true (struct :`R` 1.0 :`B` 0.019485 :`A` 1.0) 10.0))))

(event `Response Add Char on client`
  (params (ErrorMessage :type String))
  (`self.Response Add Char` ErrorMessage))

(event `self.SetMainMenuWidget`
  (params (widget :type "UserWidget Object Reference"))
  (set `self.MainMenuWidget` widget))

(event `self.RemoveWidget`
  (params (Widget :type "UserWidget Object Reference"))
  (`Widget.RemoveFromParent` Widget)
  (if (== Widget (`self.MainMenuWidget`))
    (set `self.MainMenuWidget` null)
    (elif (== Widget (`self.SelectCreateCharWidget`))
      (set `self.SelectCreateCharWidget` null)
      (elif (== Widget (`self.CreateCharWidget`))
        (set `self.CreateCharWidget` null)))))

(event `self.RequestErrorMessage`
  (params (Message :type "String (by ref)"))
  (`KismetSystemLibrary.PrintString` Message true true (struct :`R` 1.0 :`B` 0.019485 :`A` 1.0) 5.0))

(fn `AddSelectCreateCharUI`
  (returns (NewUI :type "UserWidget Object Reference"))
  (bind _returnvalue (`|CreateWidget` "/Game/L2U4/UI/2Lobby/W_SelectCreateChar.W_SelectCreateChar_C" self))
  (bind _output_get (set `self.SelectCreateCharWidget` _returnvalue))
  (return _output_get))

(fn `GetCreateCharUI`
  (returns (ReturnWidget :type "UserWidget Object Reference"))
  (return (`self.CreateCharWidget`)))

(fn `GetMainMenuUI`
  (returns (ReturnWidget :type "UserWidget Object Reference"))
  (bind _mainmenuwidget (`self.MainMenuWidget`))
  (`/Engine/EditorBlueprintResources/StandardMacros.IsValid` _mainmenuwidget
    (:`Is Valid`
      (return _mainmenuwidget))
    (:`Is Not Valid`
      (bind _returnvalue (`|CreateWidget` "/Game/L2U4/UI/2Lobby/W_MainMenu.W_MainMenu_C" self))
      (bind _output_get (set `self.MainMenuWidget` _returnvalue))
      (return _output_get))))

(fn `GetSelectCreateCharUI`
  (returns (ReturnWidget :type "UserWidget Object Reference"))
  (return (`self.SelectCreateCharWidget`)))

(fn `UserConstructionScript`
  (`parent.UserConstructionScript`))